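; BP_Weapon is a collectible weapon that deals melee and radial damage for a BP_Warrior.
; Overlapping its pickup sphere hands it to the warrior, disables the sphere and binds the warrior's radial attack event.
; Attack-check begin and end events toggle WeaponCollision, whose overlaps apply damage credited to the owner's controller.
; The bound radial attack applies area damage at the weapon's location, ignoring its owner.
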(event `self.ReceiveBeginPlay`
  (`PrimitiveComponent.SetCollisionEnabled` (`self.WeaponCollision`) "NoCollision"))

(event `self.Sphere.OnComponentBeginOverlap`
  (params (OverlappedComponent :type "PrimitiveComponent Object Reference") (OtherActor :type "Actor Object Reference") (OtherComp :type "PrimitiveComponent Object Reference") (OtherBodyIndex :type Integer) (bFromSweep :type Boolean) (SweepResult :type "HitResult Structure (by ref)"))
  (bind _asbp_warrior (cast `/Game/Blueprints/Warrior/BP_Warrior` OtherActor))
  (`/Game/Blueprints/Warrior/BP_Warrior.OnWeaponCollected` _asbp_warrior self)
  (`PrimitiveComponent.SetCollisionEnabled` (`self.Sphere`) "NoCollision")
  (add `/Game/Blueprints/Warrior/BP_Warrior.RadialAttackEvent` _asbp_warrior (delegate `RadialAttack`)))

(event `RadialAttack`
  (`/Engine/EditorBlueprintResources/StandardMacros.IsValid` (stale `self.Sphere.OnComponentBeginOverlap` _asbp_warrior)
    (:`Is Valid`
      (`GameplayStatics.ApplyRadialDamage` (`self.RadialDamage`) (`self.K2_GetActorLocation`) (`self.RadialDamageRadius`) null (`|MakeArray` (`self.GetOwner`)) self (`Pawn.GetController` (stale `self.Sphere.OnComponentBeginOverlap` _asbp_warrior))))))

(event `OnAttackCheckBegin`
  (`PrimitiveComponent.SetCollisionEnabled` (`self.WeaponCollision`) "QueryOnly"))

(event `OnAttackCheckEnd`
  (`PrimitiveComponent.SetCollisionEnabled` (`self.WeaponCollision`) "NoCollision"))

(event `self.WeaponCollision.OnComponentBeginOverlap`
  (params (OverlappedComponent :type "PrimitiveComponent Object Reference") (OtherActor :type "Actor Object Reference") (OtherComp :type "PrimitiveComponent Object Reference") (OtherBodyIndex :type Integer) (bFromSweep :type Boolean) (SweepResult :type "HitResult Structure (by ref)"))
  (bind _ascharacter (cast `Character` (`self.GetOwner`)))
  (`GameplayStatics.ApplyDamage` OtherActor (`self.Damage`) (`Pawn.GetController` _ascharacter) self))

(fn `UserConstructionScript`)