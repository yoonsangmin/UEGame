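; Player warrior character with Enhanced Input movement, camera look and melee combat using a collected weapon attached to a hand socket.
; A Locomotion/Attack/Dead state gates input, and attacks chain AM_Attack montage sections through a queued combo.
; Attack event handlers toggle weapon hit checks, add dash impulses and broadcast radial attacks.
; DamageRecevier handles health and death, feeding the HP widget, while damage drives a timeline material hit flash.
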(event `self.ReceiveBeginPlay`
  (bind _returnvalue (`GameplayStatics.GetPlayerController` 0))
  ;[1 1 1 1 36] 초기화
  (`/Engine/EditorBlueprintResources/StandardMacros.IsValid` _returnvalue
    (:`Is Valid`
      (`EnhancedInputSubsystemInterface.AddMappingContext` (pcsubsystem `EnhancedInputLocalPlayerSubsystem` _returnvalue) "/Game/Blueprints/Inputs/IMC_Character.IMC_Character" 0 (struct))
      (add `/Game/Blueprints/BP_DamageReceiver.OnDead` (`self.DamageRecevier`) (delegate `OnDead`))
      (bind _returnvalue_2 (`PrimitiveComponent.CreateDynamicMaterialInstance` (`self.Mesh`) 0 "/Game/InfinityBladeWarriors/Characters/TM/CharM_Warrior/M_Char_Warrior_Inst.M_Char_Warrior_Inst" "None"))
      (set `self.DynamicMaterialInstance` _returnvalue_2)
      (bind _aswbp_hphud (cast `/Game/UI/WBP_HPHUD` (`WidgetComponent.GetUserWidgetObject` (`self.HPBar`))))
      (set `self.HPHUD` _aswbp_hphud)
      (`PrimitiveComponent.SetCastShadow` (`self.HPBar`) false)
      (add `/Game/Blueprints/BP_DamageReceiver.OnHealthPowerChanged` (`self.DamageRecevier`) (delegate `OnHealthPowerChanged`)))))

(event `OnDead`
  (bind _returnvalue (`GameplayStatics.GetPlayerController` 0))
  ;[1 1 1 1 36] 초기화
  (`PrimitiveComponent.SetCollisionEnabled` (`self.CapsuleComponent`) "NoCollision")
  (set `self.State` "NewEnumerator2")
  (`/Engine/EditorBlueprintResources/StandardMacros.IsValid` _returnvalue
    (:`Is Valid`
      (`EnhancedInputSubsystemInterface.RemoveMappingContext` (pcsubsystem `EnhancedInputLocalPlayerSubsystem` _returnvalue) "/Game/Blueprints/Inputs/IMC_Character.IMC_Character" (struct)))))

(event `OnHealthPowerChanged`
  ;[1 1 1 1 36] 초기화
  (`/Game/UI/WBP_HPHUD.SetHPPercent` (`self.HPHUD`) (`/Game/Blueprints/BP_DamageReceiver.GetHPPercent` (`self.DamageRecevier`))))

(event `EnhancedInput|/Game/ThirdPerson/Input/Actions/IA_Move`
  (params (ActionValue :type "Vector2D Structure") (ElapsedSeconds :type "Float (double-precision)") (TriggeredSeconds :type "Float (double-precision)") (InputAction :type "InputAction Object Reference" :default "/Game/ThirdPerson/Input/Actions/IA_Move.IA_Move"))
  (bind (_returnvalue_roll _returnvalue_pitch _returnvalue_yaw) (`KismetMathLibrary.BreakRotator` (`self.GetControlRotation`)))
  ;[1 1 1 1 36] 캐릭터 이동
  (:`Triggered`
    (switch `/Game/Blueprints/Warrior/EWarriorState` (`self.State`)
      (:`NewEnumerator0`
        (`self.AddMovementInput` (+ (* (`KismetMathLibrary.GetRightVector` (`KismetMathLibrary.MakeRotator` 0.0 0.0 _returnvalue_yaw)) ActionValue_X) (* (`KismetMathLibrary.GetForwardVector` (`KismetMathLibrary.MakeRotator` 0.0 0.0 _returnvalue_yaw)) ActionValue_Y)))))))

(event `EnhancedInput|/Game/ThirdPerson/Input/Actions/IA_Jump`
  (params (ActionValue :type Boolean) (ElapsedSeconds :type "Float (double-precision)") (TriggeredSeconds :type "Float (double-precision)") (InputAction :type "InputAction Object Reference" :default "/Game/ThirdPerson/Input/Actions/IA_Jump.IA_Jump"))
  ;[1 1 1 1 36] 점프
  (:`Started`
    (switch `/Game/Blueprints/Warrior/EWarriorState` (`self.State`)
      (:`NewEnumerator0`
        (`self.Jump`)))))

(event `EnhancedInput|/Game/ThirdPerson/Input/Actions/IA_Look`
  (params (ActionValue :type "Vector2D Structure") (ElapsedSeconds :type "Float (double-precision)") (TriggeredSeconds :type "Float (double-precision)") (InputAction :type "InputAction Object Reference" :default "/Game/ThirdPerson/Input/Actions/IA_Look.IA_Look"))
  ;[1 1 1 1 36] 카메라 회전
  (:`Triggered`
    (`self.AddControllerYawInput` ActionValue_X)
    (`self.AddControllerPitchInput` ActionValue_Y)
    (switch `/Game/Blueprints/Warrior/EWarriorState` (`self.State`)
      (:`NewEnumerator1`
        (`self.TurnToTarget`)))))

(event `EnhancedInput|/Game/Blueprints/Inputs/IA_Attack`
  (params (ActionValue :type Boolean) (ElapsedSeconds :type "Float (double-precision)") (TriggeredSeconds :type "Float (double-precision)") (InputAction :type "InputAction Object Reference" :default "/Game/Blueprints/Inputs/IA_Attack.IA_Attack"))
  ;[1 1 1 1 36] 공격 입력 처리
  (:`Triggered`
    (if (`|EnumInequality` (`self.State`) "NewEnumerator2")
      (`/Engine/EditorBlueprintResources/StandardMacros.IsValid` (`self.Weapon`)
        (:`Is Valid`
          (if (not (`NavMovementComponent.IsFalling` (`self.CharacterMovement`)))
            (if (`|EnumInequality` (`self.State`) "NewEnumerator1")
              (set `self.State` "NewEnumerator1")
              (`self.PlayAnimMontage` "/Game/Blueprints/Warrior/AM_Attack.AM_Attack" 1.0 "Attack1")
              (else
                (switch `name` (`AnimInstance.Montage_GetCurrentSection` (`SkeletalMeshComponent.GetAnimInstance` (`self.Mesh`)) "/Game/Blueprints/Warrior/AM_Attack.AM_Attack")
                  (:`Attack1`
                    (set `self.NextCombo` "Attack2"))
                  (:`Attack2`
                    (set `self.NextCombo` "Attack3"))
                  (:`Attack3`
                    (set `self.NextCombo` "Attack4")))))))))))

(event `OnComboAttack`
  ;[1 1 1 1 36] 콤보
  (if (!= (`self.NextCombo`) "None")
    (`self.PlayAnimMontage` "/Game/Blueprints/Warrior/AM_Attack.AM_Attack" 1.0 (`self.NextCombo`))
    (set `self.NextCombo` "None")))

(event `OnAttackEnd`
  ;[1 1 1 1 36] 공격 종료 처리
  (set `self.State` "NewEnumerator0")
  (set `self.NextCombo` "None"))

(event `OnAttackCheckBegin`
  (bind _weapon (`self.Weapon`))
  ;[1 1 1 1 36] 공격 판정 시작/종료
  (`/Engine/EditorBlueprintResources/StandardMacros.IsValid` _weapon
    (:`Is Valid`
      (`/Game/Blueprints/Props/BP_Weapon.OnAttackCheckBegin` _weapon))))

(event `OnAttackCheckEnd`
  (bind _weapon (`self.Weapon`))
  ;[1 1 1 1 36] 공격 판정 시작/종료
  (`/Engine/EditorBlueprintResources/StandardMacros.IsValid` _weapon
    (:`Is Valid`
      (`/Game/Blueprints/Props/BP_Weapon.OnAttackCheckEnd` _weapon))))

(event `OnAttackDash`
  ;[1 1 1 1 36] 공격 시 앞으로 슬라이드
  (`CharacterMovementComponent.AddImpulse` (`self.CharacterMovement`) (* (`self.GetActorForwardVector`) (`self.DashPower`)) true))

(event `OnRadialAttack`
  ;[1 1 1 1 36] Radial 이벤트 발행
  (`self.RadialAttackEvent`))

(event `OnWeaponCollected`
  (params (Weapon :type "/Game/Blueprints/Props/BP_Weapon Object Reference"))
  (`self.SetOwner` Weapon self)
  (`/Engine/EditorBlueprintResources/StandardMacros.IsValid` (`self.Weapon`)
    (:`Is Not Valid`
      (`self.K2_AttachToComponent` Weapon (`self.Mesh`) "WeaponPosition" "SnapToTarget" "SnapToTarget" "SnapToTarget" true)
      (set `self.Weapon` Weapon))))

(event `self.ReceiveAnyDamage`
  (params (Damage :type "Float (single-precision)") (DamageType :type "DamageType Object Reference") (InstigatedBy :type "Controller Object Reference") (DamageCauser :type "Actor Object Reference"))
  (`/Game/Blueprints/BP_DamageReceiver.ReceiveDamage` (`self.DamageRecevier`) Damage)
  (`/Game/UI/WBP_HPHUD.SetHPPercent` (`self.HPHUD`) (`/Game/Blueprints/BP_DamageReceiver.GetHPPercent` (`self.DamageRecevier`)))
  (`/Game/UI/WBP_HPHUD.PlayTextAnimation` (`self.HPHUD`) (`KismetMathLibrary.FTrunc` Damage))
  (bind (_direction _hitvalue) (`Timeline|DamageEffect` :!via `PlayFromStart`)
    (:`Update`
      (`MaterialInstanceDynamic.SetScalarParameterValue` (`self.DynamicMaterialInstance`) "HitValue" _hitvalue))))

(fn `IsDead`
  (returns (IsDead :type Boolean))
  (return (`|EnumEquality` (`self.State`) "NewEnumerator2")))

(fn `TurnToTarget`
  (bind (_returnvalue_roll _returnvalue_pitch _returnvalue_yaw) (`KismetMathLibrary.BreakRotator` (`self.GetControlRotation`)))
  (`self.K2_SetActorRotation` (`KismetMathLibrary.MakeRotator` 0.0 0.0 _returnvalue_yaw)))

(fn `UserConstructionScript`)