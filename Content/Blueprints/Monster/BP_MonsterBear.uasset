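; BP_MonsterBear is a bear enemy that spots, chases and attacks the player warrior.
; Its state drives walk speed and a blackboard key; PawnSensing starts the chase, which ends when the target leaves sight radius.
; A damage receiver component updates the HP bar, with camera shake and material hit flash; death dissolves the mesh, then destroys the actor.
; An attack collision, toggled by check events, applies damage on overlap.
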(event `self.ReceiveBeginPlay`
  (bind _returnvalue (`PrimitiveComponent.CreateDynamicMaterialInstance` (`self.Mesh`) 0 "/Game/InfinityBladeAdversaries/Enemy/Enemy_Bear/Materials/M_Bear_Stone_Inst.M_Bear_Stone_Inst" "None"))
  (set `self.DynamicInstance` _returnvalue)
  (add `/Game/Blueprints/BP_DamageRecevier.OnDead` (`self.DamageRecevier`) (delegate `OnDead`))
  (bind _aswbp_hphud (cast `/Game/UI/WBP_HPHUD` (`WidgetComponent.GetUserWidgetObject` (`self.HPBar`))))
  (set `self.HPHUD` _aswbp_hphud)
  (`PrimitiveComponent.SetCollisionEnabled` (`self.AttackCollision`) "NoCollision"))

(event `OnDead`
  (`self.SetState` "NewEnumerator3")
  (`PrimitiveComponent.SetCollisionEnabled` (`self.CapsuleComponent`) "NoCollision")
  (bind (_direction _dissolve _dissolvecolor) (`Timeline|DeadEvent` :!via `PlayFromStart`)
    (:`Update`
      (`MaterialInstanceDynamic.SetScalarParameterValue` (`self.DynamicInstance`) "Dissolve" _dissolve)
      (`MaterialInstanceDynamic.SetScalarParameterValue` (`self.DynamicInstance`) "HitValue" (* _dissolve 100.0))
      (`MaterialInstanceDynamic.SetVectorParameterValue` (`self.DynamicInstance`) "HitColor" _dissolvecolor))
    (:`Finished`
      (`self.K2_DestroyActor`))))

(event `self.ReceiveActorBeginOverlap`
  (params (OtherActor :type "Actor Object Reference")))

(event `self.ReceiveAnyDamage`
  (params (Damage :type "Float (single-precision)") (DamageType :type "DamageType Object Reference") (InstigatedBy :type "Controller Object Reference") (DamageCauser :type "Actor Object Reference"))
  (`/Game/Blueprints/BP_DamageRecevier.ReceiveDamage` (`self.DamageRecevier`) Damage)
  (`/Game/UI/WBP_HPHUD.SetHPPercent` (`self.HPHUD`) (`/Game/Blueprints/BP_DamageRecevier.GetHPPercent` (`self.DamageRecevier`)))
  (`PlayerCameraManager.StartCameraShake` :`self` (`GameplayStatics.GetPlayerCameraManager` 0) :`ShakeClass` "/Game/Blueprints/Warrior/BP_Shake.BP_Shake_C")
  (bind (_direction _effectvalue) (`Timeline|HitEffect` :!via `PlayFromStart`)
    (:`Update`
      (`MaterialInstanceDynamic.SetScalarParameterValue` (`self.DynamicInstance`) "HitValue" _effectvalue))))

(event `SetState`
  (params (NewState :type "/Game/Blueprints/Monster/EBearState Enum" :default "NewEnumerator0"))
  (if (`|EnumInequality` (`self.State`) "NewEnumerator3")
    (if (`|EnumInequality` NewState (`self.State`))
      (bind _output_get (set `self.State` NewState))
      (`BlackboardComponent.SetValueAsEnum` (`AIBlueprintHelperLibrary.GetBlackboard` null) (`self.StateKey`) _output_get)
      (`|ExecutionSequence`
        (:`then_0`
          (switch `/Game/Blueprints/Monster/EBearState` (`self.State`)
            (:`NewEnumerator0`
              (set `CharacterMovementComponent.MaxWalkSpeed` 200.0 (`self.CharacterMovement`)))
            (:`NewEnumerator1`
              (set `CharacterMovementComponent.MaxWalkSpeed` 500.0 (`self.CharacterMovement`)))
            (:`NewEnumerator2`
              (set `CharacterMovementComponent.MaxWalkSpeed` 0.0 (`self.CharacterMovement`) :!label _label))
            (:`NewEnumerator3`
              (goto _label))))))))

(event `self.PawnSensing.OnSeePawn`
  (params (Pawn :type "Pawn Object Reference"))
  (if (`|EnumEquality` (`self.State`) "NewEnumerator0")
    (bind _asbp_warrior (cast `/Game/Blueprints/Warrior/BP_Warrior` Pawn))
    (if (`|EnumInequality` (`/Game/Blueprints/Warrior/BP_Warrior.State` _asbp_warrior) "NewEnumerator2")
      (`self.SetState` "NewEnumerator1")
      (bind _output_get (set `self.Instigator` Pawn))
      (`BlackboardComponent.SetValueAsObject` (`AIBlueprintHelperLibrary.GetBlackboard` (`AIBlueprintHelperLibrary.GetAIController` self)) (`self.TargetPlayerKey`) _output_get))))

(event `self.ReceiveTick`
  (params (DeltaSeconds :type "Float (single-precision)"))
  (switch `/Game/Blueprints/Monster/EBearState` (`self.State`)
    (:`NewEnumerator0`
      (`self.OnLocomotion`))
    (:`NewEnumerator1`
      (`self.OnChase`))
    (:`NewEnumerator2`
      (`self.OnAttack`))))

(event `OnLocomotion`)

(event `OnChase`
  (bind _instigator (`self.Instigator`))
  (`/Engine/EditorBlueprintResources/StandardMacros.IsValid` _instigator
    (:`Is Valid`
      (if (> (`KismetMathLibrary.Vector_Distance` (`self.K2_GetActorLocation`) (`self.K2_GetActorLocation` _instigator)) (`PawnSensingComponent.SightRadius` (`self.PawnSensing`)))
        (set `self.Instigator` null)
        (`self.SetState` "NewEnumerator0")))))

(event `OnAttack`)

(event `AttackCheckBegin`
  (`PrimitiveComponent.SetCollisionEnabled` (`self.AttackCollision`) "QueryOnly"))

(event `AttackCheckEnd`
  (`PrimitiveComponent.SetCollisionEnabled` (`self.AttackCollision`) "NoCollision"))

(event `self.AttackCollision.OnComponentBeginOverlap`
  (params (OverlappedComponent :type "PrimitiveComponent Object Reference") (OtherActor :type "Actor Object Reference") (OtherComp :type "PrimitiveComponent Object Reference") (OtherBodyIndex :type Integer) (bFromSweep :type Boolean) (SweepResult :type "HitResult Structure (by ref)"))
  (`GameplayStatics.ApplyDamage` OtherActor (`self.Damage`) (`self.GetController`) self))

(fn `UserConstructionScript`)