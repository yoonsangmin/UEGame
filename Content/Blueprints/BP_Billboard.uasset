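; BP_Billboard is a billboard scene component that keeps itself turned toward the first player's camera.
; Every Tick, it builds a world rotation with MakeRotFromXY from the camera's negated forward and right vectors, so it faces against the view direction rather than at the camera's position.
; An unconnected alternative that copies the camera rotation directly remains in the graph.
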(event `self.ReceiveTick`
  (params (DeltaSeconds :type "Float (single-precision)"))
  (bind _returnvalue (`PlayerCameraManager.GetCameraRotation` (`GameplayStatics.GetPlayerCameraManager` 0)))
  (`self.K2_SetWorldRotation` (`KismetMathLibrary.MakeRotFromXY` (* (`KismetMathLibrary.GetForwardVector` _returnvalue) -1.0) (* (`KismetMathLibrary.GetRightVector` _returnvalue) -1.0))))