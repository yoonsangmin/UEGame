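; BP_Platform is a moving platform actor that starts moving when play begins.
; It caches its starting location, then plays the Move timeline.
; Each update offsets the actor from that origin along the Arrow component's forward vector, scaled by the timeline alpha and MoveLength, without sweep.
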(event `self.ReceiveBeginPlay`
  (set `self.OriginalLocation` (`self.K2_GetActorLocation`))
  (bind (_direction _alpha) (`Timeline|Move`)
    (:`Update`
      (`self.K2_SetActorLocation` (+ (`self.OriginalLocation`) (* (* _alpha (`self.MoveLength`)) (`SceneComponent.GetForwardVector` (`self.Arrow`))))))))

(fn `UserConstructionScript`)